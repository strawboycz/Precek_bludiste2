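; BP_door is a puzzle door that removes itself when its pressure plates are pressed in numerical order.
; On BeginPlay it binds each valid plate's PlatePressed event to a counter, unbinding that plate's events when it reports in.
; The expected number advances on a match, and the door is destroyed when it reaches three.
; A plate numbered higher than expected opens the Bludiste level.
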(event `self.ReceiveBeginPlay`
  (for _array_element (`self.PressurePlates`)
    (`/Engine/EditorBlueprintResources/StandardMacros.IsValid` _array_element
      (:`Is Valid`
        (add `/Game/Blueprints/BP_pressurePlate.PlatePressed` _array_element (delegate `CountInPlate`))))))

(event `CountInPlate`
  (params (PlateNumber :type Integer) (PlateObject :type "/Game/Blueprints/BP_pressurePlate Object Reference"))
  (bind _nextplatenumber (`self.NextPlateNumber`))
  (clear `/Game/Blueprints/BP_pressurePlate.PlatePressed` PlateObject)
  (if (== PlateNumber _nextplatenumber)
    (`/Engine/EditorBlueprintResources/StandardMacros.IncrementInt` _nextplatenumber
      (:`  `
        (if (== 3 _nextplatenumber)
          (`self.K2_DestroyActor`)
          (else
            (`KismetSystemLibrary.PrintString` (`KismetStringLibrary.Conv_IntToString` _nextplatenumber))))))
    (elif (> PlateNumber _nextplatenumber)
      (`GameplayStatics.OpenLevelBySoftObjectPtr` "/Game/Levels/Bludiste.Bludiste"))))

(fn `UserConstructionScript`)